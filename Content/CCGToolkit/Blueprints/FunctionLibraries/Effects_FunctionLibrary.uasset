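; Blueprint function library that resolves and spawns particle and sound effects for card and player events in the card game.
; Card lookups map an effect state to assets in the card struct, using the wildcard index to pick the ability for ability use.
; Card health-change states and all player states have no assets assigned.
; The spawn helper places a scaled emitter at an actor or given location and plays sound in 2D.
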(fn GetCardEffectsforState
  (params (Effect :type CardEffects_Enum%20Enum :default "NewEnumerator0") (CardStruct :type Card%20Struct%20Structure) (WildcardIndex :type Integer))
  (bind _abilities (Utilities|Struct|BreakCard_Struct CardStruct))
  (bind (_attack _health _placement_settings) (Utilities|Struct|BreakCard_Struct CardStruct))
  (bind (_attack_particle _attack_soundcue) (Utilities|Struct|BreakAttack_Struct _attack))
  (bind (_dealth_particle _sound_cue_death) (Utilities|Struct|BreakHealth_Struct _health))
  (bind (_entry_particle _entry_soundcue) (Utilities|Struct|BreakPlacement_Struct _placement_settings))
  (bind _output (Utilities|Array|Get(acopy) _abilities WildcardIndex))
  (bind (_particle _soundcue) (Utilities|Struct|BreakAbility_Struct _output))
  (Utilities|FlowControl|Sequence
    (:then_0
      (if (Utilities|Enum|Equal(Enum) Effect "NewEnumerator3")
        (if (Utilities|Array|IsValidIndex (Utilities|Struct|BreakCard_Struct CardStruct) WildcardIndex)
          ;[0.631 0.3018 1 0.3] Update UE5.22 - Remove Invalid Index 0 Warnings for cards
          ;
          ; Get the Ability Particle and Audio Cue for the given effect (if valid).
          (Utilities|FlowControl|Sequence
            (:then_0
              (LocalVariables|SetOutParticle _particle))
            (:then_1
              (LocalVariables|SetOutSoundCue _soundcue))))
        (else
          ;[0.631 0.3018 1 0.3] Update UE5.22 - Remove Invalid Index 0 Warnings for cards
          ;
          ; Get the Particle and Audio Cue for the given effect (if valid).
          (Utilities|FlowControl|Sequence
            (:then_0
              (LocalVariables|SetOutParticle (Utilities|Select :Index Effect :NewEnumerator0 _entry_particle :NewEnumerator4 _attack_particle :NewEnumerator1 0 :NewEnumerator2 0 :NewEnumerator3 0 :NewEnumerator5 _dealth_particle)))
            (:then_1
              (LocalVariables|SetOutSoundCue (Utilities|Select :Index Effect :NewEnumerator0 _entry_soundcue :NewEnumerator4 _attack_soundcue :NewEnumerator1 0 :NewEnumerator2 0 :NewEnumerator3 0 :NewEnumerator5 _sound_cue_death)))))))
    (:then_1
      (return (LocalVariables|GetOutParticle) (LocalVariables|GetOutSoundCue)))))

(fn GetPlayerEffectsforState
  (params (Effect :type BoardPlayerEffects_Enum%20Enum :default "NewEnumerator0"))
  (return (Utilities|Select :Index Effect :NewEnumerator0 0 :NewEnumerator1 0 :NewEnumerator2 0) (Utilities|Select :Index Effect :NewEnumerator0 0 :NewEnumerator1 0 :NewEnumerator2 0)))

(fn SpawnParticleandSoundEffects
  (params (ParticleToSpawn :type Particle%20System%20Object%20Reference) (Location :type Vector) (OR%20ActorForLocation :type Actor%20Object%20Reference) (Scale :type Vector :default "1,1,1") (bAutoDestroy :type Boolean) (SoundCueToSpwn :type Sound%20Cue%20Object%20Reference) (Volume :type Float%20%28double-precision%29))
  (Utilities|IsValid ParticleToSpawn
    (:Is%20Valid
      (bind _returnvalue (Effects|SpawnEmitteratLocation 0 ParticleToSpawn (select (Utilities|IsValid OR%20ActorForLocation) (Transformation|GetActorLocation OR%20ActorForLocation) Location) "0, 0, 0" "1.000000,1.000000,1.000000" bAutoDestroy))
      (Transformation|SetWorldScale3D _returnvalue Scale))
    (:Is%20Not%20Valid
      _))
  (Utilities|IsValid SoundCueToSpwn
    (:Is%20Valid
      (Audio|SpawnSound2D 0 SoundCueToSpwn Volume 1.0 0.0 0))
    (:Is%20Not%20Valid
      _))
  (return))